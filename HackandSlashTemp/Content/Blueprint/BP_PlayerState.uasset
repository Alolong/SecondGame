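; BP_PlayerState holds the player's coin count and health and announces changes to them through event dispatchers.
; GetCoin increments the coin total and broadcasts it.
; AddDamage ignores hits once the player is dead, otherwise subtracts HP, broadcasts current and max HP, and fires a death dispatcher when HP reaches zero or below.
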(event `self.ReceiveTick`
  (params (DeltaSeconds :type "Float (single-precision)")))

(fn `AddDamage`
  (params (Damage :type "Float (double-precision)"))
  (if (not (`self.isDead`))
    (bind _output_get (set `self.CurHP` (- (`self.CurHP`) Damage)))
    (`self.DSUpdatePlayerHP` _output_get (`self.MaxHP`))
    (if (`self.isDead`)
      (`self.DSDeath`))))

(fn `GetCoin`
  (bind _output_get (set `self.Coiin` (+ (`self.Coiin`) 1)))
  (`self.DSCoinGet` _output_get))

(fn `isDead`
  (returns (isdeath :type Boolean))
  (return (<= (`self.CurHP`) 0.0)))

(fn `UserConstructionScript`)