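; Skill manager for an owning character that automatically casts each acquired skill whenever its cooldown elapses.
; AddSkill looks up a DT_Skill row and stores it with its timer preset to the full cooldown, so it is ready immediately.
; UpdateSkills, driven externally with delta time, advances each timer; an expired one spawns the skill's actor at the owner's transform, passing the Character, then resets.
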(fn `AddSkill`
  (params (SkillRowname :type Name))
  (bind _returnvalue (`|GetDataTableRow` "/Game/hackAndSlash/Skill/DT_Skill.DT_Skill" SkillRowname)
    (:`then`
      (bind (_name _skill _cool) (break `/Game/hackAndSlash/Skill/ST_Skill` _returnvalue))
      (`KismetArrayLibrary.Array_Add` (`self.Skills`) (make `/Game/hackAndSlash/Skill/ST_CurSkill` _returnvalue _cool))
      (`KismetSystemLibrary.PrintString` (`KismetStringLibrary.Concat_StrStr` _name) true true (struct :`G` 0.66 :`B` 1.0 :`A` 1.0) 20.0))))

(fn `DoUseSkills`
  (params (CurSkill :type "/Game/hackAndSlash/Skill/ST_CurSkill Structure"))
  (bind _returnvalue (`self.GetOwner`))
  (bind _ascharacter (cast `Character` _returnvalue))
  (`|SpawnActorFromClass` (`.Skill_9_61B7193E44F78C9F7C32D5A4A491A319` (break `/Game/hackAndSlash/Skill/ST_Skill` (`.SkillData_2_D30A785844D4DED2A74ABFAE4A5D050B` (break `/Game/hackAndSlash/Skill/ST_CurSkill` CurSkill)))) (`Actor.GetTransform` _returnvalue) "Undefined" "MultiplyWithRoot" null _ascharacter null))

(fn `UpdateSkillCooltime`
  (params (CurSkill :type "/Game/hackAndSlash/Skill/ST_CurSkill Structure (by ref)") (Deltasecond :type "Float (double-precision)"))
  ; 1.쿨타임 초 쌓기
  ; 2. 데이터의 해당 스킬 쿨타임 < 현재 돌고 있는 쿨타임 = 해당 스킬 사용
  ; 3.쿨타임 초기화
  ;; 배열로 갖고온 개별 스킬
  ;; 쿨타임 초 쌓기
  (bind _structout (setmembers `/Game/hackAndSlash/Skill/ST_CurSkill` :`StructRef` CurSkill :`CurCooltime` (+ (`.CurCooltime_5_A70A709B442C50A7CFBB03A4D29D8A27` (break `/Game/hackAndSlash/Skill/ST_CurSkill` CurSkill)) Deltasecond)))
  (bind (_skilldata _curcooltime) (break `/Game/hackAndSlash/Skill/ST_CurSkill` _structout))
  ;; 데이터의 해당 스킬 쿨타임 < 현재 돌고 있는 쿨타임 = 해당 스킬 사용
  (if (> _curcooltime (`.Cool_8_9ED15FAE4096660CFADB94B9F4E36A11` (break `/Game/hackAndSlash/Skill/ST_Skill` _skilldata)))
    (`self.DoUseSkills` _structout)
    ;; 쿨타임 초기화
    (setmembers `/Game/hackAndSlash/Skill/ST_CurSkill` :`StructRef` _structout :`CurCooltime` 0.0)))

(fn `UpdateSkills`
  (params (DeltaSeconds :type "Float (double-precision)"))
  ; 각 스킬마다 가져와 적용
  (for (_ _array_index) (`self.Skills`)
    (`self.UpdateSkillCooltime` (`|GetArrayItem` (`self.Skills`) _array_index) DeltaSeconds)))