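; Fireball skill projectile that flies forward, damages what it passes through, and destroys itself on a timer after spawn.
; Each Tick offsets the Sphere component along the actor's forward vector by Speed, without sweep.
; DoDamage accumulates delta time to throttle radial damage at the sphere's location, avoiding every-frame hits while passing through.
; The Character reference is ignored by the damage and its controller is credited as instigator.
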(event `self.ReceiveBeginPlay`
  (`KismetSystemLibrary.K2_SetTimer` null "Destroy" 5.0))

(event `self.ReceiveTick`
  (params (DeltaSeconds :type "Float (single-precision)"))
  (`|ExecutionSequence`
    (:`then_0`
      (`SceneComponent.K2_AddWorldOffset` (`self.Sphere`) (* (`self.GetActorForwardVector`) (* DeltaSeconds (`self.speed`))) false false))
    (:`then_1`
      (`self.DoDamage` DeltaSeconds))))

(fn `Destroy`
  (`self.K2_DestroyActor`))

(fn `DoDamage`
  (params (Deltasec :type "Float (double-precision)"))
  (bind _character (`self.Character`))
  ; 데미지 설정
  ;; 데미지를 통과해서 주는데 통과하는동안 연속적으로 데미지 주는 걸 방지
  (bind _output_get (set `self.DMGDelay` (+ Deltasec (`self.DMGDelay`))))
  (if (> _output_get 0.1)
    (set `self.DMGDelay` 0.0)
    ;; 폭파 데미지
    (`GameplayStatics.ApplyRadialDamage` 100.0 (`SceneComponent.K2_GetComponentLocation` (`self.Sphere`)) 50.0 null (`|MakeArray` _character :!type "Actor Object Reference") self (`Pawn.GetController` _character))))

(fn `UserConstructionScript`)