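; Item spawner component that periodically scatters random items around its owning actor.
; A looping one-second timer started on BeginPlay calls DoSpawnItem, which finds a random navigable location within a large radius of the owner.
; It picks a random row name from the DT_Item data table and spawns that row's Item class at the location.
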(event `self.ReceiveBeginPlay`
  (`KismetSystemLibrary.K2_SetTimer` null "DoSpawnItem" 1.0 true))

(fn `DoSpawnItem`
  (locals (RandomItem :type Name) (RandPosition :type "Vector Structure" :default (0.0 0.0 0.0)))
  ; 랜덤위치
  (bind _randomlocation (`NavigationSystemV1.K2_GetRandomLocationInNavigableRadius` (`Actor.K2_GetActorLocation` (`self.GetOwner`)) 10000.0 null null))
  (set `local.RandPosition` _randomlocation) ; 지역변수화
  ; 데이터 테이블
  ;; 이름 뽑기
  (bind _outrownames (`DataTableFunctionLibrary.GetDataTableRowNames` "/Game/hackAndSlash/Item/DT_Item.DT_Item"))
  ;; 랜덤지역변수(아이템명)
  (bind _output_get (set `local.RandomItem` (`KismetArrayLibrary.Array_Random` _outrownames)))
  ;; 뽑은 이름으로 데이터 가져오기
  (bind _returnvalue (`|GetDataTableRow` "/Game/hackAndSlash/Item/DT_Item.DT_Item" _output_get)
    (:`then`
      (`|SpawnActorFromClass` (`.Item_4_909037AB411C9C8495BFB8B214096616` (break `/Game/hackAndSlash/Item/ST_Item` _returnvalue)) (`KismetMathLibrary.MakeTransform` (`local.RandPosition`)) "Undefined" "MultiplyWithRoot" null null))))