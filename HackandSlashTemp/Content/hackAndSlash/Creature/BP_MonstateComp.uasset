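; BP_MonstateComp is a monster state component that tracks health, damage and death for hack-and-slash creatures.
; SetMonState loads a row from DT_Monster by name, starts current HP at the row's MaxHP and broadcasts the initial state.
; AddDamage subtracts damage while the monster is alive, then fires event dispatchers for the HP update and, once HP is zero or below, for death.
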(fn `AddDamage`
  (params (DMG :type "Float (double-precision)"))
  (bind (_currentmonsterstate_monsterstate _currentmonsterstate_curmonhp) (break `/Game/hackAndSlash/Creature/ST_CurMonState` (`self.CurrentMonsterState`)))
  (if (not (`self.isDead`))
    ; 현재 상태 변경
    (bind _structout (setmembers `/Game/hackAndSlash/Creature/ST_CurMonState` :`StructRef` (`self.CurrentMonsterState`) :`CurMonHP` (- _currentmonsterstate_curmonhp DMG)))
    ; hp갱신용
    (`self.DS_UpdateHP` (`.CurMonHP_9_7E2DCD6C46F7195E89E50D9CA8D8A7C1` (break `/Game/hackAndSlash/Creature/ST_CurMonState` _structout)) (`.MaxHP_9_E8173974430191A321955EB17203C698` (break `/Game/hackAndSlash/Creature/ST_Monster` (break `/Game/hackAndSlash/Creature/ST_CurMonState` _structout))))
    (if (`self.isDead`)
      ; 사망시 발생 이벤트
      (`self.DS_Death` (`self.CurrentMonsterState`)))))

(fn `isDead`
  (returns (isdead :type Boolean))
  (bind (_currentmonsterstate_monsterstate _currentmonsterstate_curmonhp) (break `/Game/hackAndSlash/Creature/ST_CurMonState` (`self.CurrentMonsterState`)))
  (return (<= _currentmonsterstate_curmonhp 0.0)))

(fn `SetMonState`
  (params (RowName :type Name))
  ; 최대 체력을 몬스터 현재 체력에 설정
  (bind _returnvalue (`|GetDataTableRow` "/Game/hackAndSlash/Creature/DT_Monster.DT_Monster" RowName)
    (:`then`
      (bind _output_get (set `self.CurrentMonsterState` (make `/Game/hackAndSlash/Creature/ST_CurMonState` _returnvalue (`.MaxHP_9_E8173974430191A321955EB17203C698` (break `/Game/hackAndSlash/Creature/ST_Monster` _returnvalue)))))
      ; 초깃값설정을 위함
      (`self.DS_MonState` _output_get))))