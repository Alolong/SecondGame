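; BP_MonSpawnComponent periodically spawns random monsters around its owning actor.
; After a startup delay, a looping timer runs DoSpawn, which picks a random point on a circle scaled by Radius times pi and validates it with a short downward line trace.
; It spawns a random DT_Monster row's class with BT_AITree, then passes the row name to BP_MonsterBase.SetMonState.
; Stopdospawn pauses the timer.
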(event `self.ReceiveBeginPlay`
  (`KismetSystemLibrary.Delay` 5.0)
  (`KismetSystemLibrary.K2_SetTimer` null "DoSpawn" 1.0 true))

(fn `DoSpawn`
  (locals (NewLocalVar :type "Vector Structure" :default (0.0 0.0 0.0)) (RandRowName :type Name))
  ; 원주에서 랜덤값 지역변수로 적용하여 함수 내에서 고정
  (bind _output_get (set `local.NewLocalVar` (`self.GetRandomCircleRoc`)))
  (if (`self.IsCansSpawnLoc` _output_get)
    ; 데이타 테이블 에서 이름 랜덤으로 가져와서 데이터 가져가기-
    (bind _outrownames (`DataTableFunctionLibrary.GetDataTableRowNames` "/Game/hackAndSlash/Creature/DT_Monster.DT_Monster"))
    ;; 랜덤으로 받은 값 지역변수로 셋팅하여 고정
    (bind _output_get_2 (set `local.RandRowName` (`KismetArrayLibrary.Array_Random` _outrownames)))
    (bind _returnvalue (`|GetDataTableRow` "/Game/hackAndSlash/Creature/DT_Monster.DT_Monster" _output_get_2)
      (:`then`
        ; 스폰- 새로운 곳에서 랜덤이름을 받은 몬스터를
        (bind _returnvalue_2 (`AIBlueprintHelperLibrary.SpawnAIFromClass` (`.Monster_6_3B1AC94B4B22C4AAB655A7801C1BDC4D` (break `/Game/hackAndSlash/Creature/ST_Monster` _returnvalue)) "/Game/hackAndSlash/Creature/AI/BT_AITree.BT_AITree" (`local.NewLocalVar`) (struct) false null))
        ; monsterf state에 정보 보내기
        (bind _asbp_monster_base (cast `/Game/hackAndSlash/Creature/BP_MonsterBase` _returnvalue_2))
        (`/Game/hackAndSlash/Creature/BP_MonsterBase.SetMonState` _asbp_monster_base (`local.RandRowName`))))))

(fn `GetRandomCircleRoc`
  (returns (NewParam :type "Vector Structure"))
  (locals (Rand :type "Float (double-precision)"))
  (bind _returnvalue (* (`self.radius`) 3.141592))
  ; 원의 반경 랜덤하게 구함
  (bind _output_get (set `local.Rand` (`KismetMathLibrary.RandomFloatInRange` 0.0 360.0)))
  (return (+ (`Actor.K2_GetActorLocation` (`self.GetOwner`)) (`KismetMathLibrary.MakeVector` (* (`KismetMathLibrary.Cos` _output_get) _returnvalue) (* _returnvalue (`KismetMathLibrary.Sin` _output_get))))))

(fn `IsCansSpawnLoc`
  (params (`World Loc` :type "Vector Structure"))
  (returns (IsCanSpawn :type Boolean))
  ; 스폰가능한 위치다
  ; 위치 판별
  (bind (_outhit _returnvalue) (`KismetSystemLibrary.LineTraceSingleForObjects` `World Loc` (+ `World Loc` (0.0 0.0 -100.0)) (`|MakeArray` "ObjectTypeQuery1" "ObjectTypeQuery2" :!type "EObjectTypeQuery Enum")))
  (return _returnvalue))

(fn `Stopdospawn`
  (`KismetSystemLibrary.K2_PauseTimer` null "DoSpawn"))