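; Buff component that grants timed buffs from DT_Buff rows, with Magnet as the only handled effect.
; AddBuff looks up the row, stores it with a zeroed timer and applies it by setting IsMagnet.
; Tick advances every timer, then repeatedly removes the first expired buff until none remain.
; Removing any Magnet buff clears IsMagnet, even if another is still active.
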(event `self.ReceiveTick`
  (params (DeltaSeconds :type "Float (single-precision)"))
  (`self.Updatebuff` DeltaSeconds))

(fn `AddBuff`
  (params (RowName :type Name))
  (bind _returnvalue (`|GetDataTableRow` "/Game/hackAndSlash/Item/DT_Buff.DT_Buff" RowName)
    (:`then`
      (bind _returnvalue_2 (`KismetArrayLibrary.Array_Add` (`self.Buff`) (make `/Game/hackAndSlash/Item/ST_CurBuff` _returnvalue)))
      (`KismetSystemLibrary.PrintString` (`KismetStringLibrary.Concat_StrStr` "AddBuff" (`KismetStringLibrary.Conv_NameToString` (`.Name_3_8ACE7A554F1280DDD6BFCA9DDC7587A6` (break `/Game/hackAndSlash/Item/ST_Buff` _returnvalue)))))
      (`self.UseBuff` (`|GetArrayItem` (`self.Buff`) _returnvalue_2)))))

(fn `RemoveBuff`
  (params (CurBuff :type "/Game/hackAndSlash/Item/ST_CurBuff Structure"))
  (switch `/Game/hackAndSlash/Item/EN_BuffTime` (`.Magnet_8_3276C09645D0441E0E0912AA0A89EDC5` (break `/Game/hackAndSlash/Item/ST_Buff` (break `/Game/hackAndSlash/Item/ST_CurBuff` CurBuff)))
    (:`NewEnumerator2`
      (set `self.IsMagnet` false))))

(fn `RemoveTimeOverBuff`
  (returns (RemoveIndex :type Integer))
  ; 버프제거
  (for (_array_element _array_index) (`self.Buff`)
    (bind (_buff _curcooltime) (break `/Game/hackAndSlash/Item/ST_CurBuff` _array_element))
    (if (> _curcooltime (`.CoolTime_5_3DE14AB74F032A042C7D5D8006D8282B` (break `/Game/hackAndSlash/Item/ST_Buff` _buff)))
      (`self.RemoveBuff` _array_element)
      (`KismetSystemLibrary.PrintString` (`KismetStringLibrary.Concat_StrStr` "removeBuff" (`KismetStringLibrary.Conv_NameToString` (break `/Game/hackAndSlash/Item/ST_Buff` _buff))) true true (struct :`G` 0.66 :`B` 1.0 :`A` 1.0) 20.0)
      (`KismetArrayLibrary.Array_Remove` (`self.Buff`) _array_index)
      (return _array_index)))
  (return -1))

(fn `Updatebuff`
  (params (Deltasec :type "Float (double-precision)"))
  (for (_ _array_index) (`self.Buff`)
    (`self.UpdateBuffCoolTime` (`|GetArrayItem` (`self.Buff`) _array_index) Deltasec))
  ; 쿨타임 종료된 버프 정리-무한루프?
  (bind _removeindex (`self.RemoveTimeOverBuff` :!label _label))
  (if (!= _removeindex -1)
    (goto _label)))

(fn `UpdateBuffCoolTime`
  (params (CurBuff :type "/Game/hackAndSlash/Item/ST_CurBuff Structure") (Deltasec :type "Float (double-precision)"))
  (`|ExecutionSequence`
    (:`then_0`
      (setmembers `/Game/hackAndSlash/Item/ST_CurBuff` :`StructRef` CurBuff :`CurCooltime` (+ (`.CurCooltime_6_E6CE61F94872D1B18E523ABA6F170350` (break `/Game/hackAndSlash/Item/ST_CurBuff` CurBuff)) Deltasec)))))

(fn `UseBuff`
  (params (curbuff :type "/Game/hackAndSlash/Item/ST_CurBuff Structure"))
  (`KismetSystemLibrary.PrintString` (`KismetStringLibrary.Concat_StrStr` "Usebuff" (`KismetStringLibrary.Conv_NameToString` (break `/Game/hackAndSlash/Item/ST_Buff` (break `/Game/hackAndSlash/Item/ST_CurBuff` curbuff)))))
  (switch `/Game/hackAndSlash/Item/EN_BuffTime` (`.Magnet_8_3276C09645D0441E0E0912AA0A89EDC5` (break `/Game/hackAndSlash/Item/ST_Buff` (break `/Game/hackAndSlash/Item/ST_CurBuff` curbuff)))
    (:`NewEnumerator2`
      (set `self.IsMagnet` true))))