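; BP_NameTagComp is a component that gives its owner an on-screen name tag showing a name and HP.
; It creates a BP_NameTag widget with a reference to itself on BeginPlay, adds it to the viewport, and removes it on EndPlay.
; Setter functions forward name, monster-state name and HP to the widget.
; Direct binding to BP_MonstateComp is left disconnected to keep the component reusable, and SetPlayerHP is empty.
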(event `self.ReceiveBeginPlay`
  ; 뷰포트에 위젯 올리기
  (bind _returnvalue (`|CreateWidget` "/Game/hackAndSlash/BP_NameTag.BP_NameTag_C" null self))
  (bind _output_get (set `self.Nametag` _returnvalue))
  (`UserWidget.AddToViewport` _output_get 0))

(event `self.ReceiveEndPlay`
  (params (EndPlayReason :type "EEndPlayReason Enum" :default "Destroyed"))
  (`Widget.RemoveFromParent` (`self.Nametag`)))

(fn `SetHp`
  (params (CurHP :type "Float (double-precision)") (MaxHP :type "Float (double-precision)"))
  (`/Game/hackAndSlash/BP_NameTag.SetHP` (`self.Nametag`) CurHP MaxHP))

(fn `SetName`
  (params (Name :type String))
  (`/Game/hackAndSlash/BP_NameTag.SetName` (`self.Nametag`) Name))

(fn `SetNameToWidget`
  (params (CurMonState :type "/Game/hackAndSlash/Creature/ST_CurMonState Structure"))
  ; Cur MonState의 이름을 받아 네임택 위젯에 셋하기
  (`/Game/hackAndSlash/BP_NameTag.SetName` (`self.Nametag`) (break `/Game/hackAndSlash/Creature/ST_Monster` (`.monsterstate_7_7248FD6D47A1E9385CAFB2A9940AE7E9` (break `/Game/hackAndSlash/Creature/ST_CurMonState` CurMonState)))))

(fn `SetPlayerHP`)